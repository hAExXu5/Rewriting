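; Base component for physics tools that runs an update only while its physics component is awake, for child Blueprints to override.
; Setup takes root and physics components, optionally found by name on the owner at BeginPlay.
; Wake and sleep events switch either component tick or a looping timer on and off, and each fires one zero-delta update.
; The base update calls the OnToolTick dispatcher.
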(event Custom|Setup
  (params (RootCompenent :type Scene%20Component%20Object%20Reference) (PhysicsComponent :type Primitive%20Component%20Object%20Reference))
  ;[1 1 1] Setup Event
  (Variables|Default|SetRootComponent RootCompenent)
  (Variables|Default|SetPhysicsComponent PhysicsComponent)
  (Utilities|FlowControl|Sequence
    (:then_0
      (EventDispatchers|BindEventtoOnComponentWake (Variables|Default|GetPhysicsComponent) (delegate Custom|OnComponentWake)))
    (:then_1
      (EventDispatchers|BindEventtoOnComponentSleep (Variables|Default|GetPhysicsComponent) (delegate Custom|OnComponentSleep)))
    (:then_2
      (CallFunction|SetupTimer))))

(event Custom|OnTimerUpdate
  (CallFunction|UpdateToolTick (Variables|Settings|GetTimerUpdate)))

(event Custom|SetupTimer
  ;[1 1 1] Setup Timer
  (if (Variables|Settings|GetUpdateWithEventTick)
    (if (Class|PrimitiveComponent|IsAnyRigidBodyAwake (Variables|Default|GetPhysicsComponent))
      (Components|Tick|SetComponentTickEnabled true))
    (else
      (bind _returnvalue (Utilities|Time|SetTimerbyEvent (delegate Custom|OnTimerUpdate) (Variables|Settings|GetTimerUpdate) true))
      (Variables|Default|SetTimer _returnvalue)
      (if (not (Class|PrimitiveComponent|IsAnyRigidBodyAwake (Variables|Default|GetPhysicsComponent)))
        (Utilities|Time|PauseTimerbyHandle (Variables|Default|GetTimer))))))

(event Custom|OnComponentWake
  (params (WakingComponent :type Primitive%20Component%20Object%20Reference) (BoneName :type Name))
  ;[1 1 1] Setup Event
  (if (Variables|Settings|GetUpdateWithEventTick)
    (Components|Tick|SetComponentTickEnabled true)
    (else
      (Utilities|Time|UnpauseTimerbyHandle (Variables|Default|GetTimer))))
  (CallFunction|UpdateToolTick 0.0))

(event Custom|OnComponentSleep
  (params (SleepingComponent :type Primitive%20Component%20Object%20Reference) (BoneName :type Name))
  ;[1 1 1] Setup Event
  (if (Variables|Settings|GetUpdateWithEventTick)
    (Components|Tick|SetComponentTickEnabled false)
    (else
      (Utilities|Time|PauseTimerbyHandle (Variables|Default|GetTimer))))
  (CallFunction|UpdateToolTick 0.0))

(event Custom|UpdateToolTick
  (params (DeltaSeconds :type Float%20%28single-precision%29))
  ;[1 1 1] Update Timer, will be overriden by Child Blueprints.
  (Default|CallOnToolTick))

(event EventBeginPlay
  ;[1 1 1] BeginPlay
  (if (Variables|Setup|GetAutoSetup)
    (bind _component (CallFunction|GetComponentwithName (Variables|Setup|GetRootComponentName)))
    (bind _component_2 (CallFunction|GetComponentwithName (Variables|Setup|GetPhysicsComponentName)))
    (bind _asprimitive_component (Utilities|Casting|CastToPrimitiveComponent _component_2))
    (CallFunction|Setup _component _asprimitive_component)))

(event EventTick
  (params (DeltaSeconds :type Float%20%28single-precision%29))
  ;[1 1 1] Event Tick
  (if (Variables|Settings|GetUpdateWithEventTick)
    (CallFunction|UpdateToolTick DeltaSeconds)))

(fn GetComponentwithName
  (params (Name :type String))
  (bind _array_element (Utilities|Array|ForEachLoopwithBreak (Actor|GetComponentsByClass (Components|GetOwner) "/Script/Engine.SceneComponent") :!label _label)
    (:LoopBody
      (if (Utilities|Enum|Equal(Enum) (Utilities|GetObjectName _array_element) Name)
        (Utilities|FlowControl|Sequence
          (:then_0
            (return _array_element))
          (:then_1
            (goto _label Break)))))))