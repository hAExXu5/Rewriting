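; Physics lever component for VR interactions that reports its angle and can act as an on/off switch.
; Each tool tick reads the physics component's rotation relative to the root on a chosen axis, optionally inverted, and broadcasts the value.
; Switch mode uses separate on/off thresholds for hysteresis plus an optional hold delay, firing events and attached sounds on state changes.
; Getters expose raw, normalized and switch values; debug prints remain in the tick.
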(event Custom|SetLeverState
  (params (NewOn :type Boolean))
  (bind _onsound (Variables|Default|GetOnSound))
  (bind _offsound (Variables|Default|GetOffSound))
  ;[1 1 1] Set State
  (if (Math|Boolean|NotEqual(Boolean) NewOn (Variables|Default|GetIsOn))
    (bind _output_get (Variables|Default|SetIsOn NewOn))
    (if _output_get
      (Default|CallOnLeveron)
      (Utilities|IsValid _onsound
        (:Is%20Valid
          (Audio|SpawnSoundAttached _onsound (Variables|Default|GetRootComponent) "None" "0, 0, 0" "0, 0, 0" "KeepRelativeOffset" false 1.0 1.0 0.0 0 0)))
      (else
        (Default|CallOnLeverOff)
        (Utilities|IsValid _offsound
          (:Is%20Valid
            (Audio|SpawnSoundAttached _offsound (Variables|Default|GetRootComponent) "None" "0, 0, 0" "0, 0, 0" "KeepRelativeOffset" false 1.0 1.0 0.0 0 0)))))))

(event EventBeginPlay
  ;[1 1 1] Setup
  (|CallParentFunction)
  (Variables|Default|SetLastPressChange (Math|DateTime|Now))
  (Variables|Default|SetWatchForChangeDelay (> (Variables|Default|GetPressChangeDelay) 0.01)))

(event EventUpdateToolTick
  (params (DeltaSeconds :type Float%20%28single-precision%29))
  (Utilities|FlowControl|Sequence
    (:then_0
      (Development|PrintString "1")
      (bind _output_get (Variables|Default|SetCurrentValue (CallFunction|GetToolValue)))
      (Development|PrintString "2")
      (Default|CallOnValueChange _output_get)
      (Development|PrintString "3")
      (if (Variables|Default|GetUseOnOffSwitch)
        (Development|PrintString "4")
        (if (Variables|Default|GetWatchForChangeDelay)
          ;[1 1 1] Use Delay between State changes
          (bind _output_get_2 (Variables|Default|SetTempState (> (Variables|Default|GetCurrentValue) (Math|Float|SelectFloat (Variables|Default|GetOffValue) (Variables|Default|GetOnValue) (Variables|Default|GetIsOn)))))
          (if (Math|Boolean|NotEqual(Boolean) _output_get_2 (Variables|Default|GetIsOn))
            (if (>= (Math|Float|Absolute(Float) (Math|Timespan|GetTotalSeconds (- (Variables|Default|GetLastPressChange) (Math|DateTime|Now)))) (Variables|Default|GetPressChangeDelay))
              (CallFunction|SetLeverState (Variables|Default|GetTempState))
              (Variables|Default|SetLastPressChange (Math|DateTime|Now)))
            (else
              (Variables|Default|SetLastPressChange (Math|DateTime|Now))))
          (else
            (Development|PrintString "5")
            (CallFunction|SetLeverState (> (Variables|Default|GetCurrentValue) (Math|Float|SelectFloat (Variables|Default|GetOffValue) (Variables|Default|GetOnValue) (Variables|Default|GetIsOn))))))))
    (:then_1
      (|CallParentFunction DeltaSeconds)
      (Development|PrintString "Hello"))))

(fn GetToolValue
  (bind _axis (Variables|Default|GetAxis))
  (bind _rootcomponent (Variables|Default|GetRootComponent))
  (bind _physicscomponent (Variables|Default|GetPhysicsComponent))
  (bind _returnvalue (Transformation|GetWorldRotation _physicscomponent))
  (bind _returnvalue_2 (Transformation|GetWorldTransform _rootcomponent))
  (bind _returnvalue_3 (Math|Transform|InverseTransformRotation _returnvalue_2 _returnvalue))
  (bind (_roll _pitch _yaw) (Math|Rotator|BreakRotator _returnvalue_3))
  (bind _returnvalue_4 (Utilities|Select :Index _axis :NewEnumerator0 _roll :NewEnumerator1 _pitch :NewEnumerator2 _yaw))
  (return (Math|Float|SelectFloat _returnvalue_4 (* _returnvalue_4 -1.0) (Variables|Default|GetInvertValue))))

(fn GetCurrentValue
  (bind _currentvalue (Variables|Default|GetCurrentValue))
  (return _currentvalue (Math|Float|Clamp(Float) (/ _currentvalue (Variables|Default|GetValueRange)) -1.0)))

(fn GetSwitchValue
  (return (Variables|Default|GetIsOn)))