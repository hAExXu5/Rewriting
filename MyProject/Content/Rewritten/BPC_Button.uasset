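; BPC_Button is a physical push-button component that tracks pressed state and fires press and release events with optional attached sounds.
; Each tool tick, without a change delay, it compares the physics component's root-local Z against separate press and release thresholds for hysteresis.
; With a delay set, it instead applies a temporary state, fixed to false here, once it has differed for that long.
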(event Custom|SetButtonPressedState
  (params (Pressed :type Boolean))
  (bind _presssound (Variables|Default|GetPressSound))
  (bind _releasesound (Variables|Default|GetReleaseSound))
  (if (Math|Boolean|NotEqual(Boolean) Pressed (Variables|Default|GetPressed))
    (bind _output_get (Variables|Default|SetPressed Pressed))
    (if _output_get
      (Default|CallOnButtonPress)
      (Utilities|IsValid _presssound
        (:Is%20Valid
          (Audio|SpawnSoundAttached _presssound (Variables|Default|GetRoot%20Component) "None" "0, 0, 0" "0, 0, 0" "KeepRelativeOffset" false 1.0 1.0 0.0 0 0)))
      (else
        (Default|CallOnButonRelease)
        (Utilities|IsValid _releasesound
          (:Is%20Valid
            (Audio|SpawnSoundAttached _releasesound (Variables|Default|GetRoot%20Component) "None" "0, 0, 0" "0, 0, 0" "KeepRelativeOffset" false 1.0 1.0 0.0 0 0)))))))

(event EventBeginPlay
  (|CallParentFunction)
  (Variables|Default|SetLastPressChange (Math|DateTime|Now))
  (Variables|Default|SetWatchForChangeDelay (> (Variables|Default|GetPressChangeDelay) 0.01)))

(event EventUpdateToolTick
  (params (Delta%20Seconds :type Float%20%28single-precision%29))
  (if (Variables|Default|GetWatchForChangeDelay)
    (bind _output_get (Variables|Default|SetTempPressState false))
    (if (Math|Boolean|NotEqual(Boolean) _output_get (Variables|Default|GetPressed))
      (if (>= (Math|Float|Absolute(Float) (Math|Timespan|GetTotalSeconds (- (Variables|Default|GetLastPressChange) (Math|DateTime|Now)))) (Variables|Default|GetPressChangeDelay))
        (CallFunction|SetButtonPressedState (Variables|Default|GetTempPressState))
        (Variables|Default|SetLastPressChange (Math|DateTime|Now)))
      (else
        (Variables|Default|SetLastPressChange (Math|DateTime|Now))))
    (else
      (CallFunction|SetButtonPressedState (< (.Z (Math|Vector|BreakVector (Math|Transform|InverseTransformLocation (Transformation|GetWorldTransform (Variables|Default|GetRoot%20Component)) (Transformation|GetWorldLocation (Variables|Default|GetPhysics%20Component))))) (Math|Float|SelectFloat (Variables|Default|GetReleaseZ) (Variables|Default|GetPressZ) (Variables|Default|GetPressed)))))))

(fn GetButtonPressedState
  (return (Variables|Default|GetPressed)))