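; BPC_Tools is a base actor component that runs an overridable tool update tied to a physics component's wake and sleep state.
; Setup, optionally automatic at BeginPlay via name lookup, stores root and physics components and binds wake/sleep events.
; Updates run through event tick, switched on and off with physics, or a looping timer that starts paused when asleep.
; UpdateToolTick calls OnToolTick by default.
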(event Custom|Setup
  (params (Root%20Component :type Scene%20Component%20Object%20Reference) (Physics%20Component :type Primitive%20Component%20Object%20Reference))
  (Variables|Default|SetRoot%20Component Root%20Component)
  (Variables|Default|SetPhysics%20Component Physics%20Component)
  (Utilities|FlowControl|Sequence
    (:then_0
      (EventDispatchers|BindEventtoOnComponentWake (Variables|Default|GetPhysics%20Component) (delegate Custom|OnComponentWake)))
    (:then_1
      (EventDispatchers|BindEventtoOnComponentSleep (Variables|Default|GetPhysics%20Component) (delegate Custom|OnComponentSleep)))
    (:then_2
      (CallFunction|SetupTimer))))

(event Custom|OnTimerUpdate
  ;[1 1 1] Timer
  (CallFunction|UpdateToolTick (Variables|Settings|GetTimer%20Update)))

(event Custom|OnComponentSleep
  (params (SleepingComponent :type Primitive%20Component%20Object%20Reference) (BoneName :type Name))
  (if (Variables|Settings|GetUpdateWithEventTick)
    (Components|Tick|SetComponentTickEnabled false)
    (else
      (Utilities|Time|UnpauseTimerbyHandle (Variables|Default|GetTimer))))
  (CallFunction|UpdateToolTick 0.0))

(event Custom|SetupTimer
  ;[1 1 1] Timer
  (if (Variables|Settings|GetUpdateWithEventTick)
    (if (Class|PrimitiveComponent|IsAnyRigidBodyAwake (Variables|Default|GetPhysics%20Component))
      (Components|Tick|SetComponentTickEnabled true))
    (else
      (bind _returnvalue (Utilities|Time|SetTimerbyEvent (delegate Custom|OnTimerUpdate) (Variables|Settings|GetTimer%20Update) true))
      (bind _output_get (Variables|Default|SetTimer _returnvalue))
      (if (not (Class|PrimitiveComponent|IsAnyRigidBodyAwake (Variables|Default|GetPhysics%20Component)))
        (Utilities|Time|PauseTimerbyHandle _output_get)))))

(event Custom|UpdateToolTick
  (params (Delta%20Seconds :type Float%20%28single-precision%29))
  ;[1 1 1] To be overrriden
  (Default|CallOnToolTick))

(event Custom|OnComponentWake
  (params (WakingComponent :type Primitive%20Component%20Object%20Reference) (BoneName :type Name))
  (if (Variables|Settings|GetUpdateWithEventTick)
    (Components|Tick|SetComponentTickEnabled true)
    (else
      (Utilities|Time|UnpauseTimerbyHandle (Variables|Default|GetTimer))))
  (CallFunction|UpdateToolTick 0.0))

(event EventTick
  (params (DeltaSeconds :type Float%20%28single-precision%29))
  (if (Variables|Settings|GetUpdateWithEventTick)
    (CallFunction|UpdateToolTick DeltaSeconds)))

(event EventBeginPlay
  ;[1 1 1] Begin play
  (if (Variables|Setup|GetAuto%20Setup)
    (bind _component (CallFunction|GetComponentwithName (Variables|Setup|GetRootComponentName)))
    (bind _component_2 (CallFunction|GetComponentwithName (Variables|Setup|GetPhysicsComponentName)))
    (bind _asprimitive_component (Utilities|Casting|CastToPrimitiveComponent _component))
    (CallFunction|Setup _component_2 _asprimitive_component)))

(fn GetComponentwithName
  (params (Name :type String))
  (bind _array_element (Utilities|Array|ForEachLoopwithBreak (Actor|GetComponentsByClass (Components|GetOwner) "/Script/Engine.SceneComponent") :!label _label)
    (:LoopBody
      (if (Utilities|Enum|Equal(Enum) (Utilities|GetObjectName _array_element) Name)
        (Utilities|FlowControl|Sequence
          (:then_0
            (return _array_element))
          (:then_1
            (goto _label Break)))))))